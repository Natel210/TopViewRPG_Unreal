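; Modular character Blueprint that assembles face, hair, helmet and body skeletal meshes onto one animated Mesh.
; BeginSetMesh caches current parts as defaults and clears them.
; RefreshMesh restores missing Face, Ear, Under and Lower meshes, then sets master pose, choosing FrontHair and Helmet or full Hair by Helmet component validity.
; The Glove and Boots fallbacks mistakenly check and set Lower.
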(event EventBeginPlay
  (Variables|*Default|SetDefaultCharacterFace (Utilities|Struct|MakeS_std_CharacterFace (Variables|/Script/Engine.SkinnedMeshComponent|GetSkeletalMesh (Variables|Default|GetFace)) (Variables|/Script/Engine.SkinnedMeshComponent|GetSkeletalMesh (Variables|Default|GetEar)) (Variables|/Script/Engine.SkinnedMeshComponent|GetSkeletalMesh (Variables|Default|GetHair)) (Variables|/Script/Engine.SkinnedMeshComponent|GetSkeletalMesh (Variables|Default|GetHelmet)) (Variables|/Script/Engine.SkinnedMeshComponent|GetSkeletalMesh (Variables|Default|GetFrontHair))))
  (Variables|*Default|SetDefaultCharacterBady ""))

(event Collision|EventActorBeginOverlap
  (params (OtherActor :type Actor%20Object%20Reference)))

(event EventTick
  (params (DeltaSeconds :type Float%20%28single-precision%29)))

(fn ConstructionScript)

(fn RefreshMesh
  (bind _mesh (Variables|Character|GetMesh))
  (CallFunction|ChackValidFace)
  (CallFunction|ChackValidBady)
  (|CheckHelmet
    (:Is%20Valid
      (|EqHelmetMasterPose _mesh))
    (:Is%20Not%20Valid
      (|UnEqHelmetMasterPose _mesh))))

(fn ChackValidFace
  (bind _face (Variables|Default|GetFace))
  (bind _ear (Variables|Default|GetEar))
  (Utilities|IsValid (Variables|/Script/Engine.SkinnedMeshComponent|GetSkeletalMesh _face)
    (:Is%20Valid
      _)
    (:Is%20Not%20Valid
      (Class|SkinnedMeshComponent|SetSkeletalMesh _face (.*Face (Utilities|Struct|BreakS_std_CharacterFace (Variables|*Default|GetDefaultCharacterFace))) true)))
  (Utilities|IsValid (Variables|/Script/Engine.SkinnedMeshComponent|GetSkeletalMesh _ear)
    (:Is%20Not%20Valid
      (Class|SkinnedMeshComponent|SetSkeletalMesh _ear (.*Ear (Utilities|Struct|BreakS_std_CharacterFace (Variables|*Default|GetDefaultCharacterFace))) true))))

(fn ChackValidBady
  (bind _lower (Variables|Default|GetLower))
  (bind _under (Variables|Default|GetUnder))
  (bind _lower_2 (Variables|Default|GetLower))
  (bind _lower_3 (Variables|Default|GetLower))
  ;[1 1 1] Check Under
  (Utilities|IsValid (Variables|/Script/Engine.SkinnedMeshComponent|GetSkeletalMesh _under)
    (:Is%20Valid
      _)
    (:Is%20Not%20Valid
      (Class|SkinnedMeshComponent|SetSkeletalMesh _under (.*Under (Utilities|Struct|BreakS_std_CharacterBady (Variables|*Default|GetDefaultCharacterBady))) true)))
  ;[1 1 1] Check Lower
  (Utilities|IsValid (Variables|/Script/Engine.SkinnedMeshComponent|GetSkeletalMesh _lower_2)
    (:Is%20Valid
      _)
    (:Is%20Not%20Valid
      (Class|SkinnedMeshComponent|SetSkeletalMesh _lower_2 (.*Lower (Utilities|Struct|BreakS_std_CharacterBady (Variables|*Default|GetDefaultCharacterBady))) true)))
  ;[1 1 1] Check Glove
  (Utilities|IsValid (Variables|/Script/Engine.SkinnedMeshComponent|GetSkeletalMesh _lower_3)
    (:Is%20Valid
      _)
    (:Is%20Not%20Valid
      (Class|SkinnedMeshComponent|SetSkeletalMesh _lower_3 (.*Glove (Utilities|Struct|BreakS_std_CharacterBady (Variables|*Default|GetDefaultCharacterBady))) true)))
  ;[1 1 1] Check Glove
  (Utilities|IsValid (Variables|/Script/Engine.SkinnedMeshComponent|GetSkeletalMesh _lower)
    (:Is%20Valid
      _)
    (:Is%20Not%20Valid
      (Class|SkinnedMeshComponent|SetSkeletalMesh _lower (.*Boots (Utilities|Struct|BreakS_std_CharacterBady (Variables|*Default|GetDefaultCharacterBady))) true)))
  (return))

(fn BeginSetMesh
  ;[1 1 1] Set Defualt
  ;;[1 1 1] Face
  (Variables|*Default|SetDefaultCharacterFace (Utilities|Struct|MakeS_std_CharacterFace (Variables|/Script/Engine.SkinnedMeshComponent|GetSkeletalMesh (Variables|Default|GetFace)) (Variables|/Script/Engine.SkinnedMeshComponent|GetSkeletalMesh (Variables|Default|GetEar)) (Variables|/Script/Engine.SkinnedMeshComponent|GetSkeletalMesh (Variables|Default|GetHair)) (Variables|/Script/Engine.SkinnedMeshComponent|GetSkeletalMesh (Variables|Default|GetHelmet)) (Variables|/Script/Engine.SkinnedMeshComponent|GetSkeletalMesh (Variables|Default|GetFrontHair))))
  ;;[1 1 1] Bady
  (Variables|*Default|SetDefaultCharacterBady (Utilities|Struct|MakeS_std_CharacterBady (Variables|/Script/Engine.SkinnedMeshComponent|GetSkeletalMesh (Variables|Default|GetUnder)) (Variables|/Script/Engine.SkinnedMeshComponent|GetSkeletalMesh (Variables|Default|GetLower)) (Variables|/Script/Engine.SkinnedMeshComponent|GetSkeletalMesh (Variables|Default|GetGlove)) (Variables|/Script/Engine.SkinnedMeshComponent|GetSkeletalMesh (Variables|Default|GetBoots)) (Variables|/Script/Engine.SkinnedMeshComponent|GetSkeletalMesh (Variables|Default|GetBelt))))
  ;[1 1 1] Clear
  ;;[1 1 1] Face
  (Class|SkinnedMeshComponent|SetSkeletalMesh (Variables|Default|GetFace) 0 true)
  (Class|SkinnedMeshComponent|SetSkeletalMesh (Variables|Default|GetEar) 0 true)
  (Class|SkinnedMeshComponent|SetSkeletalMesh (Variables|Default|GetHair) 0 true)
  (Class|SkinnedMeshComponent|SetSkeletalMesh (Variables|Default|GetHelmet) 0 true)
  (Class|SkinnedMeshComponent|SetSkeletalMesh (Variables|Default|GetFrontHair) 0 true)
  ;;[1 1 1] Bady
  (Class|SkinnedMeshComponent|SetSkeletalMesh (Variables|Default|GetUnder) 0 true)
  (Class|SkinnedMeshComponent|SetSkeletalMesh (Variables|Default|GetLower) 0 true)
  (Class|SkinnedMeshComponent|SetSkeletalMesh (Variables|Default|GetGlove) 0 true)
  (Class|SkinnedMeshComponent|SetSkeletalMesh (Variables|Default|GetBoots) 0 true)
  (Class|SkinnedMeshComponent|SetSkeletalMesh (Variables|Default|GetBelt) 0 true))